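; BP_MyHouse is a Blueprint scripting sandbox built around a procedurally assembled house.
; EventBuildHouse adds static mesh components at runtime, scaling and placing cubes as foundation and walls and two ramps as the roof.
; BeginPlay only prints a message through EventDoStuff; the build call, variable printing and AddTwoNumbers test sit in disconnected chains.
; EventAnimateHouse and the construction script are empty, and HelloWorld is an unused print function.
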(event Custom|EventDoStuff
  (params (WhatToDo :type String))
  (Development|PrintString WhatToDo))

(event Custom|EventAnimateHouse)

(event Custom|EventBuildHouse
  ;[0.15 0.15 0.15 0.5] Foundation
  (Development|PrintString "starting construction")
  (bind _returnvalue (AddComponent|AddStaticMeshComponent false))
  (Components|StaticMesh|SetStaticMesh _returnvalue "/Game/LevelPrototyping/Meshes/SM_Cube.SM_Cube")
  (Transformation|SetRelativeLocation _returnvalue "0.000000,0.000000,-10.000000" false false)
  (Transformation|SetRelativeScale3D _returnvalue "1.200000,1.200000,0.100000")
  ;[0.15 0.15 0.15 0.5] Wall
  (bind _returnvalue_2 (AddComponent|AddStaticMeshComponent false))
  (Components|StaticMesh|SetStaticMesh _returnvalue_2 "/Game/LevelPrototyping/Meshes/SM_Cube.SM_Cube")
  (Transformation|SetRelativeLocation _returnvalue_2 "0, 0, 0" false false)
  (Transformation|SetRelativeScale3D _returnvalue_2 "0.100000,1.000000,1.000000")
  ;[0.15 0.15 0.15 0.5] Wall
  (bind _returnvalue_3 (AddComponent|AddStaticMeshComponent false))
  (Components|StaticMesh|SetStaticMesh _returnvalue_3 "/Game/LevelPrototyping/Meshes/SM_Cube.SM_Cube")
  (Transformation|SetRelativeLocation _returnvalue_3 "110.000000,0.000000,0.000000" false false)
  (Transformation|SetRelativeScale3D _returnvalue_3 "0.100000,1.000000,1.000000")
  ;[0.15 0.15 0.15 0.5] Wall
  (bind _returnvalue_4 (AddComponent|AddStaticMeshComponent false))
  (Components|StaticMesh|SetStaticMesh _returnvalue_4 "/Game/LevelPrototyping/Meshes/SM_Cube.SM_Cube")
  (Transformation|SetRelativeLocation _returnvalue_4 "110.000000,90.000000,0.000000" false false)
  (Transformation|SetRelativeRotation _returnvalue_4 "0.000000,90.000000,0.000000" false false)
  (Transformation|SetRelativeScale3D _returnvalue_4 "0.100000,1.000000,1.000000")
  ;[0.15 0.15 0.15 0.5] Wall
  (bind _returnvalue_5 (AddComponent|AddStaticMeshComponent false))
  (Components|StaticMesh|SetStaticMesh _returnvalue_5 "/Game/LevelPrototyping/Meshes/SM_Cube.SM_Cube")
  (Transformation|SetRelativeLocation _returnvalue_5 "110.000000,0.000000,0.000000" false false)
  (Transformation|SetRelativeRotation _returnvalue_5 "0.000000,90.000000,0.000000" false false)
  (Transformation|SetRelativeScale3D _returnvalue_5 "0.100000,1.000000,1.000000")
  ;[0.15 0.15 0.15 0.5] Roof1
  (bind _returnvalue_6 (AddComponent|AddStaticMeshComponent false))
  (Components|StaticMesh|SetStaticMesh _returnvalue_6 "/Game/LevelPrototyping/Meshes/SM_Ramp.SM_Ramp")
  (Transformation|SetRelativeLocation _returnvalue_6 "60.000000,100.000000,100.000000" false false)
  (Transformation|SetRelativeRotation _returnvalue_6 "0.000000,-90.000000,0.000000" false false)
  (Transformation|SetRelativeScale3D _returnvalue_6 "1.000000,0.750000,0.800000")
  ;[0.15 0.15 0.15 0.5] Roof2
  (bind _returnvalue_7 (AddComponent|AddStaticMeshComponent false))
  (Components|StaticMesh|SetStaticMesh _returnvalue_7 "/Game/LevelPrototyping/Meshes/SM_Ramp.SM_Ramp")
  (Transformation|SetRelativeLocation _returnvalue_7 "60.000000,0.000000,100.000000" false false)
  (Transformation|SetRelativeRotation _returnvalue_7 "0.000000,90.000000,0.000000" false false)
  (Transformation|SetRelativeScale3D _returnvalue_7 "1.000000,0.750000,0.800000"))

(event EventBeginPlay
  (CallFunction|EventDoStuff "Jump up and down"))

(fn ConstructionScript)

(fn HelloWorld
  (Development|PrintString "Hello"))

(fn AddTwoNumbers
  (params (FirstNumber :type Float%20%28double-precision%29) (SecondNumber :type Float%20%28double-precision%29))
  (return (+ FirstNumber SecondNumber)))